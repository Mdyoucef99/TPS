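; BP_Enemy is an enemy character with hit points that can be damaged and destroyed.
; Its Damage function decrements HP, destroys the actor at zero, and otherwise writes the passed object to the EnemyActor Blackboard key for its AI.
; Overlapping a ThirdPersonCharacter deactivates its CharacterMovement, with no reactivation in this Blueprint.
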(event EventBeginPlay)

(event Collision|EventActorBeginOverlap
  (params (OtherActor :type Actor%20Object%20Reference))
  (Utilities|Casting|CastToThirdPersonCharacter OtherActor)
  (Components|Activation|SetActive (Variables|Character|GetCharacterMovement) false false))

(event EventTick
  (params (DeltaSeconds :type Float%20%28single-precision%29)))

(fn ConstructionScript)

(fn Damage
  (params (ObjectValue :type Object%20Object%20Reference))
  (bind _result (Math|Integer|DecrementInt (Variables|Default|GetHP))
    (:%20%20
      (if (== _result 0)
        (Actor|DestroyActor)
        (else
          (AI|Components|Blackboard|SetValueasObject (AI|GetBlackboard self) (Utilities|Name|MakeLiteralName "EnemyActor") ObjectValue))))))